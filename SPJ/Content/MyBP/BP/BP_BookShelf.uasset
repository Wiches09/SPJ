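; BP_BookShelf is a bookshelf hazard that topples over and ends the game when it hits the player.
; The Falling event plays a timeline whose track is added each update as local roll to the Pivot component.
; Rotation is skipped while the Collision component overlaps the player.
; When that component begins overlapping BP_FirstPersonCharacterNew, it calls GameOver on the character.
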(event OnComponentBeginOverlap(collision)
  (params (OverlappedComponent :type Primitive%20Component%20Object%20Reference) (OtherActor :type Actor%20Object%20Reference) (OtherComp :type Primitive%20Component%20Object%20Reference) (OtherBodyIndex :type Integer) (bFromSweep :type Boolean) (SweepResult :type Hit%20Result%20Structure%20%28by%20ref%29))
  (bind _asbp_first_person_character_new (Utilities|Casting|CastToBP_FirstPersonCharacterNew OtherActor))
  (Default|GameOver _asbp_first_person_character_new))

(event Custom|Falling
  (bind _returnvalue (Game|GetPlayerCharacter 0))
  (bind _falling_track (Timeline|Timeline Play)
    (:Update
      (Utilities|Casting|CastToBP_FirstPersonCharacterNew _returnvalue)
      (if (not (Collision|IsOverlappingActor (Variables|Default|Getcollision) _returnvalue :!class /Script/Engine.PrimitiveComponent))
        (Transformation|AddLocalRotation (Variables|Default|Getpivot) (Math|Rotator|MakeRotator _falling_track 0.0 0.0) false false)))))

(fn ConstructionScript)