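; BP_NewWaterFiller2 is an interactable water filler that refills the player's status through the status widget.
; A Box overlap sets an in-range flag and, on entry, caches the first-person character and binds Interact to its interact dispatcher.
; Interact calls Refill on that widget by a fixed amount only while in range, then prints a debug string.
; The binding is never removed on exit, so the flag alone gates it.
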(event OnComponentBeginOverlap(Box)
  (params (OverlappedComponent :type Primitive%20Component%20Object%20Reference) (OtherActor :type Actor%20Object%20Reference) (OtherComp :type Primitive%20Component%20Object%20Reference) (OtherBodyIndex :type Integer) (bFromSweep :type Boolean) (SweepResult :type Hit%20Result%20Structure%20%28by%20ref%29))
  ;[0.15 0.15 0.15 0.5] Interact
  (Variables|Default|SetIsInRange true)
  (bind _asbp_first_person_character_new_2 (Utilities|Casting|CastToBP_FirstPersonCharacterNew2 (Game|GetPlayerCharacter 0)))
  (bind _output_get (Variables|Default|SetPlayerRef _asbp_first_person_character_new_2))
  (EventDispatchers|BindEventtoInteractDispatcher _output_get (delegate Custom|Interact)))

(event OnComponentEndOverlap(Box)
  (params (OverlappedComponent :type Primitive%20Component%20Object%20Reference) (OtherActor :type Actor%20Object%20Reference) (OtherComp :type Primitive%20Component%20Object%20Reference) (OtherBodyIndex :type Integer))
  ;[0.15 0.15 0.15 0.5] Interact
  (Variables|Default|SetIsInRange false))

(event Custom|Interact
  ;[0.15 0.15 0.15 0.5] Interact
  (if (Variables|Default|GetIsInRange)
    (Default|Refill (Variables|/Game/65070201/BP/BP_FirstPersonCharacterNew2.BP_FirstPersonCharacterNew2_C|GetStatus%20Widget%20Ref (Variables|Default|GetPlayerRef)) 5.0)
    (Development|PrintString "Hello")))

(fn ConstructionScript)